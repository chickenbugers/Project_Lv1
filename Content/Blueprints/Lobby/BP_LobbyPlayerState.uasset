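; Player state for lobby players that keeps the lobby HUD in sync and handles being kicked by the server.
; It refreshes the local BP_LobbyHUD one tick after BeginPlay and again when destroyed.
; CopyProperties carries the nickname over to a BP_PlayerState.
; The Client_KickedByServer event destroys the session and, on completion, opens the Title level.
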(event Custom|OnDestroyed_Event
  (params (DestroyedActor :type Actor%20Object%20Reference))
  (Class|LobbyPlayerState|RefreshLobbyUI))

(event Custom|Client_KickedByServer
  (|DestroySession (Game|GetPlayerController 0)
    (:then
      (Game|OpenLevel(byObjectReference) "/Game/Maps/Title.Title"))))

(event EventBeginPlay
  (Utilities|FlowControl|DelayUntilNextTick)
  (Class|LobbyPlayerState|RefreshLobbyUI)
  (Game|BindEventtoOnDestroyed (delegate Custom|OnDestroyed_Event)))

(event EventCopyProperties
  (params (NewPlayerState :type Player%20State%20Object%20Reference))
  (|CallParentFunction NewPlayerState)
  (bind _asbp_player_state (Utilities|Casting|CastToBP_PlayerState NewPlayerState))
  (Variables|/Game/Blueprints/Game/Characters/Player/BP_PlayerState.BP_PlayerState_C|SetNickName _asbp_player_state (Variables|Default|GetNickName)))

(event EventRefreshLobbyUI
  (bind _returnvalue (Game|GetPlayerController 0))
  (Utilities|IsValid _returnvalue
    (:Is%20Valid
      (bind _asbp_lobby_hud (Utilities|Casting|CastToBP_LobbyHUD (HUD|GetHUD _returnvalue)))
      (Default|RefreshUI _asbp_lobby_hud))))

(fn ConstructionScript)