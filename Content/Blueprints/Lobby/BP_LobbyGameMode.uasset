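; BP_LobbyGameMode runs the multiplayer lobby, naming each joining player "User N" and launching the match once all players are ready.
; SetLevel maps the chosen map to a level name, defaulting to WaterWheel, and publishes it in the session's MAP_NAME setting.
; TryStartGame starts the advanced session, then seamlessly ServerTravels to that level.
; SaveConfig applies the map choice and stores clamped player and bot limits on BP_GameInstance.
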(event Custom|Set%20Level
  (params (InLevelName :type String))
  (Utilities|FlowControl|Sequence
    (:then_0
      (switch string InLevelName
        (:Default
          (Variables|Default|Set%20LevelName "Level_WaterWheel" :!label _label))
        (:Fountain
          (Variables|Default|Set%20LevelName "Level_Fountain"))
        (:Watermill
          (goto _label))))
    (:then_1
      (bind _extrasettings (Class|AdvancedSessionsLibrary|GetSessionSettings)
        (:OnSuccess
          (bind _modifiedsettingsarray (Class|AdvancedSessionsLibrary|AddorModifyExtraSettings _extrasettings (Utilities|Array|MakeArray (Class|AdvancedSessionsLibrary|MakeLiteralSessionPropertyString "MAP_NAME" InLevelName))))
          (|UpdateSession _modifiedsettingsarray 10 0 false false false true false true))))))

(event EventPostLogin
  (params (NewPlayer :type Player%20Controller%20Object%20Reference))
  (bind _asbp_lobby_player_state (Utilities|Casting|CastToBP_LobbyPlayerState (Variables|/Script/Engine.Controller|GetPlayerState NewPlayer)))
  (bind _result (Math|Integer|IncrementInt (Variables|Default|GetNickNameIndex))
    (:%20%20
      (Variables|/Game/Blueprints/Lobby/BP_LobbyPlayerState.BP_LobbyPlayerState_C|SetNickName _asbp_lobby_player_state (Utilities|Text|FormatText "User {0}" _result)))))

(event EventBeginPlay
  (Variables|Default|SetbUseSeamlessTravel true)
  (CallFunction|SetLevel "Fountain"))

(event EventTryStartGame
  (if (CallFunction|IsEverybodyReady)
    (|StartAdvancedSession
      (:OnSuccess
        (Development|ExecuteConsoleCommand (Utilities|String|Append "ServerTravel" " " (Variables|Default|Get%20LevelName)) 0)))))

(fn ConstructionScript)

(fn IsEverybodyReady
  (for _array_element (Variables|/Script/Engine.GameStateBase|GetPlayerArray (Game|GetGameState))
    (bind _asbp_lobby_player_state (Utilities|Casting|CastToBP_LobbyPlayerState _array_element))
    (if (not (Variables|/Game/Blueprints/Lobby/BP_LobbyPlayerState.BP_LobbyPlayerState_C|GetReady _asbp_lobby_player_state))
      (return false)))
  (return true))

(fn SaveConfig
  (params (InLevelName :type String) (InMaxPlayerCount :type Integer) (InMaxBotCount :type Integer))
  (Utilities|FlowControl|Sequence
    (:then_0
      (bind _asbp_game_instance (Utilities|Casting|CastToBP_GameInstance (Game|GetGameInstance)))
      (LocalVariables|SetBPGameInstance _asbp_game_instance))
    (:then_1
      (CallFunction|SetLevel InLevelName))
    (:then_2
      (Variables|/Game/Blueprints/BP_GameInstance.BP_GameInstance_C|SetMaxPlayerCount (LocalVariables|GetBPGameInstance) (Math|Integer|Clamp(Integer) InMaxPlayerCount 2 10)))
    (:then_3
      (Variables|/Game/Blueprints/BP_GameInstance.BP_GameInstance_C|SetMaxBotCount (LocalVariables|GetBPGameInstance) (Math|Integer|Clamp(Integer) InMaxBotCount 10 30)))))